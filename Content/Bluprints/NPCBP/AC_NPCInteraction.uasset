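; NPC interaction component that handles look-at detection and opens input for Artimus's dialogue.
; InteractWith creates the WBP_ArtimusDialougeTwo widget, without adding it to the viewport, then sets UI-only input and shows the cursor.
; InteractionTrace sphere-traces from the player's forward vector, offset by location times InteractionRange, caching LookAtActor and printing its LookAtMessage when the target changes.
; LookAt is an empty-string stub.
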(event `InteractWith`
  (params (PlayerCharacter :type "/Game/Bluprints/PlayerBP/BP_Player Object Reference"))
  (bind _returnvalue (`|CreateWidget` "/Game/Bluprints/Widgets/WBP_ArtimusDialougeTwo.WBP_ArtimusDialougeTwo_C"))
  (`WidgetBlueprintLibrary.SetInputMode_UIOnlyEx` null _returnvalue)
  (set `PlayerController.bShowMouseCursor` true (`PlayerState.GetPlayerController` (`Pawn.PlayerState` PlayerCharacter))))

(fn `InteractionTrace`
  (bind _returnvalue (`GameplayStatics.GetPlayerCharacter` 0))
  (bind _returnvalue_2 (`Actor.GetActorForwardVector` _returnvalue))
  (bind (_outhit _returnvalue_3) (`KismetSystemLibrary.SphereTraceSingle` _returnvalue_2 (+ _returnvalue_2 (* (`Actor.K2_GetActorLocation` _returnvalue) (`self.InteractionRange`))) 30.0 "TraceTypeQuery1" false (`|MakeArray` (`Actor.GetOwner` (`self.Player Character`)))))
  (if _returnvalue_3
    (bind (_bblockinghit _binitialoverlap _time _distance _location _impactpoint _normal _impactnormal _physmat _hitactor) (`GameplayStatics.BreakHitResult` _outhit))
    (if (!= _hitactor (`self.LookAtActor`))
      (bind _output_get (set `self.LookAtActor` _hitactor))
      (bind _message (message `/Game/Bluprints/PlayerBP/I_Interaction.LookAt` _output_get))
      (`KismetSystemLibrary.PrintString` (`KismetTextLibrary.Conv_TextToString` _message)))
    (else
      (set `self.LookAtActor` null))))

(fn `LookAt`
  (returns (Message :type Text))
  (return ""))